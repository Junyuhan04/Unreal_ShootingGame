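; BP_Bullet is a projectile actor that damages the boss on contact.
; Tick moves it in a straight line by adding Direction times Speed, scaled by delta time, to its location, without sweeping.
; When its Collision component overlaps a BP_Boss, it calls TakeDamage with a fixed amount and destroys itself.
; Other overlaps are ignored, and the graph has no lifetime handling.
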(event OnComponentBeginOverlap(Collision)
  (params (OverlappedComponent :type Primitive%20Component%20Object%20Reference) (OtherActor :type Actor%20Object%20Reference) (OtherComp :type Primitive%20Component%20Object%20Reference) (OtherBodyIndex :type Integer) (bFromSweep :type Boolean) (SweepResult :type Hit%20Result%20Structure%20%28by%20ref%29))
  (bind _asbp_boss (Utilities|Casting|CastToBP_Boss OtherActor))
  (Default|TakeDamage _asbp_boss 1e+01)
  (Actor|DestroyActor))

(event EventBeginPlay)

(event EventTick
  (params (DeltaSeconds :type Float%20%28single-precision%29))
  ;[0.15 0.15 0.15 0.5] 이동한다.
  (Transformation|SetActorLocation (+ (* DeltaSeconds (* (Variables|Default|GetDirection) (Variables|Default|GetSpeed))) (Transformation|GetActorLocation)) false false))

(fn ConstructionScript)