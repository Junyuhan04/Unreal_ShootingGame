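; Player actor for a shooter that moves in the Y-Z plane by swept Tick offsets from axis input and fires BP_Bullet actors it owns.
; It creates the HUD, updating the health bar on damage and the score text as points arrive.
; Reaching a score threshold spawns BP_Boss once, while zero health calls GameOver on BP_GameMode and destroys the player.
; Escape pauses with WBP_Pause or resumes, switching input mode and cursor.
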(event EventBeginPlay
  ;[0.15 0.15 0.15 0.5] UI
  (bind _returnvalue (UserInterface|CreateWidget "/Game/Blueprints/WBP/WBP_HUD.WBP_HUD_C"))
  (Variables|Default|SetHUDWidget _returnvalue)
  (UserInterface|Viewport|AddtoViewport _returnvalue 0)
  (Progress|SetPercent (Variables|/Game/Blueprints/WBP/WBP_HUD.WBP_HUD_C|GetHPBar (Variables|Default|GetHUDWidget)) (/ (Math|Conversions|ToFloat(Integer) (Variables|Default|GetHP)) (Math|Conversions|ToFloat(Integer) (Variables|Default|GetMaxHP)))))

(event EventTick
  (params (DeltaSeconds :type Float%20%28single-precision%29))
  ;[0.15 0.15 0.15 0.5] 이동한다.
  (Transformation|SetActorLocation (+ (* DeltaSeconds (* (Variables|Default|GetDirection) (Variables|Default|GetSpeed))) (Transformation|GetActorLocation)) true false))

(event Input|ActionEvents|InputActionFire
  (params (Key :type Key%20Structure :default "None"))
  (:Pressed
    (CallFunction|FireBullet)
    (Audio|PlaySound2D "/Game/Resource/Sounds/star-wars-blaster.star-wars-blaster" 1.0 1.0 0.0 0 0)))

(event Input|AxisEvents|InputAxisHorizontal
  (params (AxisValue :type Float%20%28single-precision%29))
  ;[0.15 0.15 0.15 0.5] 방향구하기
  (Variables|Default|SetDirection (Math|Vector|MakeVector 0.0 AxisValue (stale Input|AxisEvents|InputAxisVertical AxisValue))))

(event Input|AxisEvents|InputAxisVertical
  (params (AxisValue :type Float%20%28single-precision%29))
  ;[0.15 0.15 0.15 0.5] 방향구하기
  (Variables|Default|SetDirection (Math|Vector|MakeVector 0.0 (stale Input|AxisEvents|InputAxisHorizontal AxisValue) AxisValue)))

(event Input|KeyboardEvents|Escape
  (params (Key :type Key%20Structure :default "None"))
  (bind _returnvalue (Game|GetPlayerController 0))
  (bind _returnvalue_2 (Game|GetPlayerController 0))
  (:Pressed
    (if (Game|IsGamePaused)
      (Game|SetGamePaused false)
      (Input|SetInputModeGameOnly _returnvalue_2 false)
      (Variables|/Script/Engine.PlayerController|SetbShowMouseCursor _returnvalue_2 false)
      (else
        (Game|SetGamePaused true)
        (bind _returnvalue_3 (UserInterface|CreateWidget "/Game/Blueprints/WBP/WBP_Pause.WBP_Pause_C"))
        (UserInterface|Viewport|AddtoViewport _returnvalue_3 0)
        (Input|SetInputModeUIOnly _returnvalue _returnvalue_3 "DoNotLock" false)
        (Variables|/Script/Engine.PlayerController|SetbShowMouseCursor _returnvalue true)))))

(fn ConstructionScript)

(fn FireBullet
  (bind _returnvalue (Game|SpawnActorfromClass "/Game/Blueprints/BP_Bullet.BP_Bullet_C" (Math|Transform|MakeTransform (Transformation|GetWorldLocation (Variables|Default|GetFirePosition)) "0, 0, 0" "1.000000,1.000000,1.000000") "AlwaysSpawn" "MultiplyWithRoot" 0 0))
  (Variables|/Game/Blueprints/BP_Bullet.BP_Bullet_C|SetOwnerPlayer _returnvalue self))

(fn AddScore
  (params (Value :type Integer))
  (Variables|Default|SetScore (+ (Variables|Default|GetScore) Value))
  (Utilities|IsValid (Variables|Default|GetHUDWidget)
    (:Is%20Valid
      (Rendering|Components|TextRender|SetText (Variables|/Game/Blueprints/WBP/WBP_HUD.WBP_HUD_C|GetScoreText (Variables|Default|GetHUDWidget)) (Utilities|Text|ToText(Integer) (Variables|Default|GetScore)))
      (if (and (>= (Variables|Default|GetScore) 100) (not (Variables|Default|GetBossSpawned)))
        ;[0.15 0.15 0.15 0.5] Class에 보스 넣어줘야됨
        (Game|SpawnActorfromClass "/Game/Blueprints/BP_Boss.BP_Boss_C" (Math|Transform|MakeTransform "0.000000,0.000000,500.000000") "Undefined" "MultiplyWithRoot" 0 0)
        (Variables|Default|SetBossSpawned true)))))

(fn TakeDamage
  (params (Damage :type Integer))
  ;[0.15 0.15 0.15 0.5] HP -= Damage
  (Variables|Default|SetHP (- (Variables|Default|GetHP) Damage))
  ;[0.15 0.15 0.15 0.5] HP UI 표시
  (Progress|SetPercent (Variables|/Game/Blueprints/WBP/WBP_HUD.WBP_HUD_C|GetHPBar (Variables|Default|GetHUDWidget)) (/ (Math|Conversions|ToFloat(Integer) (Variables|Default|GetHP)) (Math|Conversions|ToFloat(Integer) (Variables|Default|GetMaxHP))))
  (Audio|PlaySound2D "/Game/Resource/Sounds/Player_Damaged.Player_Damaged" 1.0 1.0 0.0 0 0)
  ;[0.15 0.15 0.15 0.5] Player 죽음 처리
  (if (<= (Variables|Default|GetHP) 0)
    ;;[0.15 0.15 0.15 0.5] BP_GameMode에서 GameOver 호출
    (bind _asbp_game_mode (Utilities|Casting|CastToBP_GameMode (Game|GetGameMode)))
    (Default|GameOver _asbp_game_mode)
    (Actor|DestroyActor)))