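; BP_Boss is a boss enemy that patrols side to side, shoots on a timer and ends the game in a clear when defeated.
; Tick moves it along Y, flipping direction past fixed bounds, while a looping timer spawns Enemy_Bullet from the muzzle.
; On BeginPlay it hands itself to its HP widget.
; TakeDamage lowers HP with explosion effects, then calls GameClear on the game mode and destroys it at zero.
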(event Custom|Fire
  ;[0.15 0.15 0.15 0.5] 보스 총 발사
  (Game|SpawnActorfromClass "/Game/Blueprints/Enemy_Bullet.Enemy_Bullet_C" (Transformation|GetWorldTransform (Variables|Default|GetMuzzle)) "Undefined" "MultiplyWithRoot" 0 0))

(event Custom|TakeDamage
  (params (Damage :type Float%20%28double-precision%29))
  (Variables|Default|SetBossHP (- (Variables|Default|GetBossHP) Damage))
  (Niagara|SpawnSystematLocation "/Game/Fire_EXP_Vol01_Free/Niagara/EXP/NS_Sub_EXP_Large_001_01.NS_Sub_EXP_Large_001_01" (Transformation|GetActorLocation))
  (Audio|PlaySound2D "/Game/Resource/Sounds/Explosion.Explosion" 1.0 1.0 0.0 0 0)
  (if (<= (Variables|Default|GetBossHP) 0.0)
    (bind _asbp_game_mode (Utilities|Casting|CastToBP_GameMode (Game|GetGameMode)))
    (Default|GameClear _asbp_game_mode)
    (Actor|DestroyActor)))

(event EventTick
  (params (DeltaSeconds :type Float%20%28single-precision%29))
  (bind _returnvalue (Transformation|GetActorLocation))
  (bind _y (Math|Vector|BreakVector _returnvalue))
  (if (or (> _y 5.8e+02) (< _y -5.8e+02))
    (Variables|Default|SetDirection (* (Variables|Default|GetDirection) -1.0)))
  (Transformation|AddActorWorldOffset (Math|Vector|MakeVector 0.0 (* DeltaSeconds (* (Variables|Default|GetSpeed) (Variables|Default|GetDirection))) 0.0)))

(event EventBeginPlay
  ;[0.15 0.15 0.15 0.5] 보스 총 발사
  (Utilities|FlowControl|Sequence
    (:then_0
      (Utilities|Time|SetTimerbyEvent (delegate Custom|Fire) 5.0 true))
    (:then_1
      (bind _aswbp_boss_ui (Utilities|Casting|CastToWBP_BossUI (UserInterface|GetUserWidgetObject (Variables|Default|GetBossHPWidget))))
      (Variables|/Game/Blueprints/WBP/WBP_BossUI.WBP_BossUI_C|SetBoss _aswbp_boss_ui self))))

(fn ConstructionScript)